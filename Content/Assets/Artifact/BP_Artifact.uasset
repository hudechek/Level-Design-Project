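; BP_Artifact is a pickup actor that floats and spins until the player collects it.
; A looping timer set on BeginPlay periodically restarts a timeline, which lerps the mesh's relative height and rotation for the bob and full-turn spin.
; On Interact, it casts the first player character to PlayerCharacter, sets its HasArtifact flag and destroys itself.
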(event Custom|FloatAndSpin
  (bind _artifactmesh (Variables|Default|GetArtifactMesh))
  (bind (_direction _flaot_up_and_down _spin) (Timeline|Timeline PlayFromStart)
    (:Update
      (Transformation|SetRelativeLocation _artifactmesh (Math|Vector|Lerp(Vector) "0, 0, 0" "0.000000,0.000000,10.000000" _flaot_up_and_down) false false)
      (Transformation|SetRelativeRotation _artifactmesh (Math|Rotator|Lerp(Rotator) "0, 0, 0" "0.000000,360.000000,0.000000" _spin) false false))))

(event EventBeginPlay
  (Utilities|Time|SetTimerbyFunctionName 0 "FloatAndSpin" 6.0 true))

(event EventInteract
  ;[1 1 1] on interaction call, calls player character for variable HasArtifact and sets to true then destroys actor
  (bind _asplayer_character (Utilities|Casting|CastToPlayerCharacter (Game|GetPlayerCharacter 0)))
  (Variables|/Game/PlayerCharcter/PlayerCharacter.PlayerCharacter_C|SetHasArtifact? _asplayer_character true)
  (Actor|DestroyActor))

(fn ConstructionScript)