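; Pressure-plate puzzle button, a child Blueprint, that unlocks its target doorway while pressed.
; Box overlap by the player, or by a physics pickup whose ButtonSelection is this button, sets the unlock flag and plays a timeline lowering Cube1.
; End overlap by the player or any physics-simulating component relocks the doorway and reverses the timeline, without checking for remaining occupants.
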(event OnComponentEndOverlap(Box)
  (params (OverlappedComponent :type Primitive%20Component%20Object%20Reference) (OtherActor :type Actor%20Object%20Reference) (OtherComp :type Primitive%20Component%20Object%20Reference) (OtherBodyIndex :type Integer))
  (Utilities|Casting|CastToPlayerCharacter OtherActor
    (:then
      (Variables|/Game/Assets/DoorWay/Doorway.Doorway_C|SetIsUnlocked (Variables|Default|GetDoorWayTarget) false :!label _label)
      (bind _newtrack_0 (Timeline|Timeline_0 Reverse)
        (:Update
          (Transformation|SetRelativeLocation (Variables|Default|GetCube1) (Math|Vector|MakeVector 0.0 0.0 (Math|Float|Lerp 1e+01 0.0 _newtrack_0)) false false))))
    (:CastFailed
      (if (Physics|IsSimulatingPhysics OtherComp "None")
        (goto _label)))))

(event OnComponentBeginOverlap(Box)
  (params (OverlappedComponent :type Primitive%20Component%20Object%20Reference) (OtherActor :type Actor%20Object%20Reference) (OtherComp :type Primitive%20Component%20Object%20Reference) (OtherBodyIndex :type Integer) (bFromSweep :type Boolean) (SweepResult :type Hit%20Result%20Structure%20%28by%20ref%29))
  (Utilities|Casting|CastToPlayerCharacter OtherActor
    (:then
      (Variables|/Game/Assets/DoorWay/Doorway.Doorway_C|SetIsUnlocked (Variables|Default|GetDoorWayTarget) true :!label _label)
      (bind _newtrack_0 (Timeline|Timeline_0 Play)
        (:Update
          (Transformation|SetRelativeLocation (Variables|Default|GetCube1) (Math|Vector|MakeVector 0.0 0.0 (Math|Float|Lerp 1e+01 0.0 _newtrack_0)) false false))))
    (:CastFailed
      (bind _asbp_physics_pickup (Utilities|Casting|CastToBP_PhysicsPickup OtherActor))
      (if (== (Variables|/Game/Puzzle/BP_PhysicsPickup.BP_PhysicsPickup_C|GetButtonSelection _asbp_physics_pickup) self)
        (goto _label)))))

(fn ConstructionScript
  (|CallParentFunction))